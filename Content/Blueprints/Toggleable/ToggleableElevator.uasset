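; Toggleable elevator that raises a mover through a procedurally built shaft when turned on and reverses it when turned off.
; The construction script derives height from the floor count and stacks instanced wall meshes per floor, leaving the front open at the bottom and top.
; A timeline scales its percent by that height, with play rate set at BeginPlay from velocity over height so speed is independent of shaft height.
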(event `/Game/Blueprints/Interfaces/ToggleableObject.TurnOn`
  (bind (_direction _percent) (`Timeline|AnimElevate` :!label _label)
    (:`Update`
      (`SceneComponent.K2_SetRelativeLocation` (`self.Mover`) (`KismetMathLibrary.MakeVector` 0.0 0.0 (* _percent (`self.Max Height`))) false false))))

(event `/Game/Blueprints/Interfaces/ToggleableObject.TurnOff`
  (goto _label :!via `Reverse`))

(event `self.ReceiveBeginPlay`
  ;[1 1 1] set init playrate
  (`TimelineComponent.SetPlayRate` (`self.AnimElevate`) (/ (`self.Elevator Velocity`) (`self.Max Height`))))

(fn `UserConstructionScript`
  (locals (`Current Floor` :type Integer) (`Current Z` :type "Float (double-precision)"))
  (bind _current_floor (`local.Current Floor`))
  (set `self.Max Height` (* (`self.Max Floor`) 400.0))
  (for _index (range (+ (`self.Max Floor`) 1))
    (bind _output_get (set `local.Current Floor` _index))
    (set `local.Current Z` (* _output_get 400.0))
    ;[1 1 1] rightwall
    (`InstancedStaticMeshComponent.AddInstance` (`self.Wall Instance Mesh`) (`KismetMathLibrary.MakeTransform` (`KismetMathLibrary.MakeVector` -200.0 210.0 (`local.Current Z`))))
    ;[1 1 1] leftwall
    (`InstancedStaticMeshComponent.AddInstance` (`self.Wall Instance Mesh`) (`KismetMathLibrary.MakeTransform` (`KismetMathLibrary.MakeVector` -200.0 -210.0 (`local.Current Z`))))
    ;[1 1 1] backwall
    (`InstancedStaticMeshComponent.AddInstance` (`self.Wall Instance Mesh`) (`KismetMathLibrary.MakeTransform` (`KismetMathLibrary.MakeVector` 210.0 -200.0 (`local.Current Z`)) (struct :`Yaw` 90.0)))
    ;[1 1 1] frontwall
    (if (not (or (== (`self.Max Floor`) _current_floor) (== _current_floor 0)))
      (`InstancedStaticMeshComponent.AddInstance` (`self.Wall Instance Mesh`) (`KismetMathLibrary.MakeTransform` (`KismetMathLibrary.MakeVector` -200.0 -200.0 (`local.Current Z`)) (struct :`Yaw` 90.0))))))