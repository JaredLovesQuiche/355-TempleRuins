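; Interactive door that the first-person player toggles open and closed with the Interact input, enabled on the actor at BeginPlay.
; Two trigger components track whether the player is in front or behind, selecting which timeline yaws the door, scaled by OpenAngle.
; State flags remember the side used, so the next press reverses that timeline; closing has no proximity check.
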(event `self.Opener0.OnComponentBeginOverlap`
  (params (OverlappedComponent :type "PrimitiveComponent Object Reference") (OtherActor :type "Actor Object Reference") (OtherComp :type "PrimitiveComponent Object Reference") (OtherBodyIndex :type Integer) (bFromSweep :type Boolean) (SweepResult :type "HitResult Structure (by ref)"))
  ;[1 1 1] Character Input
  (cast `/Game/Blueprints/Character/FirstPersonCharacter` OtherActor)
  (set `self.PlayerInFront` true))

(event `self.ReceiveBeginPlay`
  (`self.EnableInput` (`GameplayStatics.GetPlayerController` 0)))

(event `self.Opener0.OnComponentEndOverlap`
  (params (OverlappedComponent :type "PrimitiveComponent Object Reference") (OtherActor :type "Actor Object Reference") (OtherComp :type "PrimitiveComponent Object Reference") (OtherBodyIndex :type Integer))
  ;[1 1 1] Character Input
  (cast `/Game/Blueprints/Character/FirstPersonCharacter` OtherActor)
  (set `self.PlayerInFront` false))

(event `InputAction|Interact`
  (params (Key :type "Key Structure"))
  (:`Pressed`
    ;[1 1 1] Open/Close Door
    (if (`self.Closed`)
      (if (`self.PlayerInFront`)
        (set `self.DoorOpenF` true)
        (set `self.Closed` false)
        (bind (_direction _percent) (`Timeline|DoorOpenFront` :!label _label)
          (:`Update`
            (`SceneComponent.K2_SetRelativeRotation` (`self.Door`) (`KismetMathLibrary.MakeRotator` 0.0 0.0 (* _percent (`self.OpenAngle`))) false false)))
        (elif (`self.PlayerInBack`)
          (set `self.DoorOpenB` true)
          (set `self.Closed` false)
          (bind (_direction_2 _percent_2) (`Timeline|DoorOpenBack` :!label _label_2)
            (:`Update`
              (`SceneComponent.K2_SetRelativeRotation` (`self.Door`) (`KismetMathLibrary.MakeRotator` 0.0 0.0 (* _percent_2 (`self.OpenAngle`))) false false)))))
      (elif (`self.DoorOpenF`)
        (set `self.DoorOpenF` false)
        (set `self.Closed` true)
        (goto _label :!via `Reverse`)
        (elif (`self.DoorOpenB`)
          (set `self.DoorOpenB` false)
          (set `self.Closed` true)
          (goto _label_2 :!via `Reverse`))))))

(event `self.Opener1.OnComponentBeginOverlap`
  (params (OverlappedComponent :type "PrimitiveComponent Object Reference") (OtherActor :type "Actor Object Reference") (OtherComp :type "PrimitiveComponent Object Reference") (OtherBodyIndex :type Integer) (bFromSweep :type Boolean) (SweepResult :type "HitResult Structure (by ref)"))
  ;[1 1 1] Character Input
  (cast `/Game/Blueprints/Character/FirstPersonCharacter` OtherActor)
  (set `self.PlayerInBack` true))

(event `self.Opener1.OnComponentEndOverlap`
  (params (OverlappedComponent :type "PrimitiveComponent Object Reference") (OtherActor :type "Actor Object Reference") (OtherComp :type "PrimitiveComponent Object Reference") (OtherBodyIndex :type Integer))
  ;[1 1 1] Character Input
  (cast `/Game/Blueprints/Character/FirstPersonCharacter` OtherActor)
  (set `self.PlayerInBack` false))

(fn `UserConstructionScript`)