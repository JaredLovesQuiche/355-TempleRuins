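; Pressure plate that switches a connected actor on while something overlaps its box collider and off once the collider is empty.
; Begin overlap sends TurnOnMessage to ConnectedActor and plays the PushDown timeline, which offsets the Scene component along its relative Y axis.
; End overlap re-runs the on path if actors remain, otherwise clears On, sends TurnOffMessage and reverses the timeline.
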(event `self.Box Collider.OnComponentBeginOverlap`
  (params (OverlappedComponent :type "PrimitiveComponent Object Reference") (OtherActor :type "Actor Object Reference") (OtherComp :type "PrimitiveComponent Object Reference") (OtherBodyIndex :type Integer) (bFromSweep :type Boolean) (SweepResult :type "HitResult Structure (by ref)"))
  (bind _returnvalue (`SceneComponent.GetRelativeTransform` (`self.Scene`)))
  (message `/Game/Blueprints/Interfaces/ToggleableObject.TurnOn` (`self.ConnectedActor`) :!label _label)
  (bind (_direction _percent) (`Timeline|PushDown` :!label _label_2)
    (:`Update`
      (`SceneComponent.K2_SetRelativeLocation` (`self.Scene`) (`KismetMathLibrary.MakeVector` (.x (.location _returnvalue)) (* _percent -10.0) (.z (.location _returnvalue))) false false))))

(event `self.Box Collider.OnComponentEndOverlap`
  (params (OverlappedComponent :type "PrimitiveComponent Object Reference") (OtherActor :type "Actor Object Reference") (OtherComp :type "PrimitiveComponent Object Reference") (OtherBodyIndex :type Integer))
  (if (> (`KismetArrayLibrary.Array_Length` (`PrimitiveComponent.GetOverlappingActors` (`self.Box Collider`) null)) 0)
    (goto _label)
    (else
      (set `self.On` false)
      (message `/Game/Blueprints/Interfaces/ToggleableObject.TurnOff` (`self.ConnectedActor`))
      (goto _label_2 :!via `Reverse`))))

(fn `UserConstructionScript`)