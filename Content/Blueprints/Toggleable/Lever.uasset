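; Lever is an interactable toggle that switches a connected actor on or off.
; Each player interaction flips its On state and sends a turn-on or turn-off message to ConnectedActor.
; A LeverPullDown timeline plays forward or in reverse, rolling the Scene component up to 90 degrees while keeping its pitch and yaw.
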(event `/Game/Blueprints/Interfaces/PlayerCanInteract.Player Wants To Interact`
  (params (Player :type "/Game/Blueprints/Character/FirstPersonCharacter Object Reference"))
  (bind _connectedactor (`self.ConnectedActor`))
  (bind _returnvalue (`SceneComponent.GetRelativeTransform` (`self.Scene`)))
  (bind _output_get (set `self.On` (not (`self.On`))))
  (if _output_get
    (message `/Game/Blueprints/Interfaces/ToggleableObject.TurnOn` _connectedactor)
    (bind (_direction _percent) (`Timeline|LeverPullDown` :!label _label)
      (:`Update`
        (`SceneComponent.K2_SetRelativeRotation` (`self.Scene`) (`KismetMathLibrary.MakeRotator` (* _percent 90.0) (.pitch (.rotation _returnvalue)) (.yaw (.rotation _returnvalue))) false false)))
    (else
      (message `/Game/Blueprints/Interfaces/ToggleableObject.TurnOff` _connectedactor)
      (goto _label :!via `Reverse`))))

(fn `UserConstructionScript`)