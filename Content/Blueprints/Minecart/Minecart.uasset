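; Rideable minecart pawn that carries its own spline track and is driven forward or backward along it by the player.
; The construction script tiles spline meshes along the track.
; Each tick integrates position from velocity (explicit Euler), updates clamped velocity from input without friction, then places the Mover on the spline.
; Boarding possesses the cart and destroys the character; Interact spawns and possesses a new FirstPersonCharacter at the camera.
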(event `InputAxis|Turn` :overrideparent false
  (params (AxisValue :type "Float (single-precision)"))
  ;[1 1 1] Comment
  (`self.AddControllerYawInput` AxisValue))

(event `InputAction|MInecart Forward`
  (params (Key :type "Key Structure"))
  (:`Pressed`
    (set `self.PlayerWantsToMoveForward` true))
  (:`Released`
    (set `self.PlayerWantsToMoveForward` false)))

(event `self.ReceiveTick`
  (params (DeltaSeconds :type "Float (single-precision)"))
  (`self.Euler Step` DeltaSeconds)
  (`self.Accelerate` DeltaSeconds)
  (`self.PositionCart`))

(event `InputAxis|LookUp` :overrideparent false
  (params (AxisValue :type "Float (single-precision)"))
  ;[1 1 1] Comment
  (`self.AddControllerPitchInput` AxisValue))

(event `InputAction|Minecart Backward`
  (params (Key :type "Key Structure"))
  (:`Pressed`
    (set `self.PlayerWantsToMoveBackward` true))
  (:`Released`
    (set `self.PlayerWantsToMoveBackward` false)))

(event `/Game/Blueprints/PlayerCanInteract.Player Wants To Interact`
  (params (Player :type "/Game/Blueprints/FirstPersonCharacter Object Reference"))
  ;[1 1 1] Comment
  (`Controller.Possess` (`self.GetController` Player) self)
  (`self.K2_DestroyActor` Player))

(event `InputAction|Interact`
  (params (Key :type "Key Structure"))
  (bind _returnvalue (`SceneComponent.K2_GetComponentToWorld` (`self.Camera`)))
  (:`Pressed`
    (bind _returnvalue_2 (`|SpawnActorFromClass` "/Game/Blueprints/FirstPersonCharacter.FirstPersonCharacter_C" (`KismetMathLibrary.MakeTransform` (.location _returnvalue) (`KismetMathLibrary.MakeRotator` 0.0 0.0 (.yaw (.rotation _returnvalue)))) "Undefined" "OverrideRootScale" (`self.GetOwner`) null))
    (`Controller.Possess` (`self.GetController`) _returnvalue_2)))

(fn `Accelerate`
  (params (dt :type "Float (double-precision)"))
  (locals (dir :type "Float (double-precision)"))
  (bind _max_velocity (`self.Max Velocity`))
  (if (`self.PlayerWantsToMoveForward`)
    (set `local.dir` 1.0))
  (if (`self.PlayerWantsToMoveBackward`)
    (set `local.dir` (- (`local.dir`) 1.0)))
  (set `self.Velocity` (`KismetMathLibrary.FClamp` (+ (`self.Velocity`) (* (`local.dir`) dt (`self.Acceleration`))) (* _max_velocity -1.0) _max_velocity)))

(fn `Euler Step`
  (params (dt :type "Float (double-precision)"))
  (set `self.PositionOnSpline` (`KismetMathLibrary.FClamp` (+ (`self.PositionOnSpline`) (* dt (`self.Velocity`))) 0.0 (`SplineComponent.GetSplineLength` (`self.Spline`)))))

(fn `PositionCart`
  (bind _spline (`self.Spline`))
  (bind _positiononspline (`self.PositionOnSpline`))
  (`SceneComponent.K2_SetRelativeLocationAndRotation` (`self.Mover`) (`SplineComponent.GetLocationAtDistanceAlongSpline` _spline _positiononspline "Local") (`SplineComponent.GetRotationAtDistanceAlongSpline` _spline _positiononspline "Local") false false))

(fn `UserConstructionScript`
  (bind _spline (`self.Spline`))
  (bind _spline_2 (`self.Spline`))
  (`self.PositionCart`)
  (for _index (range (`KismetMathLibrary.FTrunc` (/ (`SplineComponent.GetSplineLength` (`self.Spline`)) (`self.LengthOfPiece`))))
    (bind _returnvalue (`AddComponent|NODE_AddSplineMeshComponent-0`))
    (bind _returnvalue_2 (* _index (`self.LengthOfPiece`)))
    (bind _returnvalue_3 (* (+ _index 1) (`self.LengthOfPiece`)))
    (`SplineMeshComponent.SetStartAndEnd` _returnvalue (`SplineComponent.GetLocationAtDistanceAlongSpline` _spline_2 _returnvalue_2 "Local") (`KismetMathLibrary.ClampVectorSize` (`SplineComponent.GetTangentAtDistanceAlongSpline` _spline_2 _returnvalue_2 "Local") 0.0 (`self.LengthOfPiece`)) (`SplineComponent.GetLocationAtDistanceAlongSpline` _spline _returnvalue_3 "Local") (`KismetMathLibrary.ClampVectorSize` (`SplineComponent.GetTangentAtDistanceAlongSpline` _spline _returnvalue_3 "Local") 0.0 (`self.LengthOfPiece`)) true)))