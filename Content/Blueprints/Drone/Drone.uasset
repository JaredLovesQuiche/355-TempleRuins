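; Player-possessable drone pawn, flown by applying physics forces to its Mover component.
; Input pushes it along the camera's flattened forward vector, its right vector and world Z, while look input drives controller rotation.
; While possessed and falling without axis input, Tick scales its whole velocity by ManualDamping.
; Interacting possesses the drone and destroys the player character; pressing Interact again spawns and possesses a new FirstPersonCharacter at the camera.
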(event `InputAxis|Turn` :overrideparent false
  (params (AxisValue :type "Float (single-precision)"))
  ;[1 1 1] Camera Controls
  (`self.AddControllerYawInput` AxisValue))

(event `InputAxis|MoveForward`
  (params (AxisValue :type "Float (single-precision)"))
  (bind (_returnvalue_x _returnvalue_y) (`KismetMathLibrary.BreakVector` (`SceneComponent.GetForwardVector` (`self.Camera`))))
  ;[1 1 1] Movement
  (`PrimitiveComponent.AddForce` (`self.Mover`) (* (`KismetMathLibrary.Normal` (`KismetMathLibrary.MakeVector` _returnvalue_x _returnvalue_y)) (* AxisValue (`self.MovementForce`))) "None" false))

(event `InputAxis|LookUp` :overrideparent false
  (params (AxisValue :type "Float (single-precision)"))
  ;[1 1 1] Camera Controls
  (`self.AddControllerPitchInput` AxisValue))

(event `InputAxis|MoveRight`
  (params (AxisValue :type "Float (single-precision)"))
  ;[1 1 1] Movement
  (`PrimitiveComponent.AddForce` (`self.Mover`) (* (`SceneComponent.GetRightVector` (`self.Camera`)) (* AxisValue (`self.MovementForce`))) "None" false))

(event `InputAxis|MoveUp`
  (params (AxisValue :type "Float (single-precision)"))
  ;[1 1 1] Movement
  (`PrimitiveComponent.AddForce` (`self.Mover`) (`KismetMathLibrary.MakeVector` 0.0 0.0 (* AxisValue (`self.MovementForce`))) "None" false))

(event `self.ReceiveTick`
  (params (DeltaSeconds :type "Float (single-precision)"))
  (bind _mover (`self.Mover`))
  ;[1 1 1] Restrict Y Velocity when possessed
  (bind _returnvalue (`PrimitiveComponent.GetPhysicsLinearVelocity` (`self.Mover`) "None"))
  (if (and (`self.IsPossessed`) (== (stale `InputAxis|MoveUp` AxisValue) 0.0) (< (.z _returnvalue) 0.0))
    (bind _returnvalue_2 (`PrimitiveComponent.GetPhysicsLinearVelocity` _mover "None"))
    (`PrimitiveComponent.SetPhysicsLinearVelocity` _mover (* _returnvalue_2 (`self.ManualDamping`)) false "None")))

(event `/Game/Blueprints/PlayerCanInteract.Player Wants To Interact`
  (params (Player :type "/Game/Blueprints/FirstPersonCharacter Object Reference"))
  ;[1 1 1] Possess
  (`Controller.Possess` (`self.GetController` Player) self)
  (`self.K2_DestroyActor` Player)
  (set `self.IsPossessed` true))

(event `InputAction|Interact`
  (params (Key :type "Key Structure"))
  (bind _returnvalue (`SceneComponent.K2_GetComponentToWorld` (`self.Camera`)))
  ;[1 1 1] Cancel Possession
  (:`Pressed`
    (bind _returnvalue_2 (`|SpawnActorFromClass` "/Game/Blueprints/FirstPersonCharacter.FirstPersonCharacter_C" (`KismetMathLibrary.MakeTransform` (.location _returnvalue) (`KismetMathLibrary.MakeRotator` 0.0 0.0 (.yaw (.rotation _returnvalue)))) "Undefined" "OverrideRootScale" (`self.GetOwner`) null))
    (`Controller.Possess` (`self.GetController`) _returnvalue_2)
    (set `self.IsPossessed` false)))

(fn `UserConstructionScript`)