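; An LED light Blueprint that cycles its color through red, green and blue each time its Trigger event fires.
; The construction script creates a dynamic material instance from LEDMat on the NeonLight component, stores it back in LEDMat and applies the current color.
; Trigger advances CurrentState and calls UpdateMaterialColor, which maps the state to a color for a vector parameter, though the parameter name is left as None.
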(event `/Game/Blueprints/Interfaces/Triggerable.Trigger`
  (switch `/Game/Blueprints/LEDLight/LEDColor` (`self.Current State`)
    (:`NewEnumerator0`
      (set `self.Current State` "NewEnumerator1"))
    (:`NewEnumerator1`
      (set `self.Current State` "NewEnumerator2"))
    (:`NewEnumerator2`
      (set `self.Current State` "NewEnumerator0")))
  (`self.UpdateMaterialColor`))

(fn `UpdateMaterialColor`
  (`MaterialInstanceDynamic.SetVectorParameterValue` (`self.LEDMat`) "None" (select `/Game/Blueprints/LEDLight/LEDColor` (`self.Current State`) :`NewEnumerator0` (struct :`R` 1.0 :`A` 1.0) :`NewEnumerator1` (struct :`G` 1.0 :`A` 1.0) :`NewEnumerator2` (struct :`B` 1.0 :`A` 1.0) :!type "LinearColor Structure")))

(fn `UserConstructionScript`
  (bind _returnvalue (`PrimitiveComponent.CreateDynamicMaterialInstance` (`self.Neon Light`) 0 "/Game/Blueprints/LEDLight/LEDMat.LEDMat" "None"))
  (set `self.LEDMat` _returnvalue)
  (`self.UpdateMaterialColor`))