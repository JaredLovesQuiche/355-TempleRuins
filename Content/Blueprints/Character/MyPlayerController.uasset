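; Player controller that creates the HUD widget and adds it to the viewport on BeginPlay.
; BeginPlay first casts and stores the MyGameInstance, stopping before HUD creation if the cast fails; the stored reference is otherwise unused.
; Destroyed removes TheHUD if valid, but the node assigning the new widget to TheHUD is disconnected, so this graph never sets that reference.
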(event `self.ReceiveBeginPlay`
  (bind _asmy_game_instance (cast `/Game/Blueprints/Character/MyGameInstance` (`GameplayStatics.GetGameInstance`)))
  (set `self.theGameInstance` _asmy_game_instance)
  (bind _returnvalue (`|CreateWidget` "/Game/Blueprints/GUI/HUD.HUD_C"))
  (`UserWidget.AddToViewport` _returnvalue 0))

(event `self.ReceiveDestroyed`
  (bind _thehud (`self.theHUD`))
  (`/Engine/EditorBlueprintResources/StandardMacros.IsValid` _thehud
    (:`Is Valid`
      (`Widget.RemoveFromParent` _thehud))))

(fn `UserConstructionScript`)